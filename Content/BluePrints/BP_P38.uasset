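; BP_P38 is a P-38 plane Blueprint that flies forward continuously while spinning its two propellers.
; Each Tick moves the actor along its local X axis by MoveSpeed, then calls RotatePropeller for Left and Right, both scaled by delta time.
; RotatePropeller adds relative roll to the given component at PropellerRotateSpeed.
; Steering is not implemented: Pitch input only prints its axis value and Roll is empty.
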(event `self.ReceiveBeginPlay`)

(event `self.ReceiveTick`
  (params (DeltaSeconds :type "Float (single-precision)"))
  (`|ExecutionSequence`
    (:`then_0`
      ;[1 1 1] 앞으로 이동
      (`self.K2_AddActorLocalOffset` (`KismetMathLibrary.MakeVector` (* (`GameplayStatics.GetWorldDeltaSeconds`) (`self.MoveSpeed`)))))
    (:`then_1`
      ;[1 1 1] 왼쪽 프로펠러 회전
      (`self.Rotate Propeller` (`self.Left`)))
    (:`then_2`
      ;[1 1 1] 오른쪽 프로펠러 회전
      (`self.Rotate Propeller` (`self.Right`)))))

(event `InputAxis|Pitch`
  (params (AxisValue :type "Float (single-precision)"))
  (`KismetSystemLibrary.PrintString` (`KismetStringLibrary.Conv_DoubleToString` AxisValue)))

(event `InputAxis|Roll`
  (params (AxisValue :type "Float (single-precision)")))

(fn `Rotate Propeller`
  (params (Where :type "StaticMeshComponent Object Reference"))
  (`SceneComponent.K2_AddRelativeRotation` Where (`KismetMathLibrary.MakeRotator` (* (`GameplayStatics.GetWorldDeltaSeconds`) (`self.PropellerRotateSpeed`))) false false))

(fn `UserConstructionScript`)