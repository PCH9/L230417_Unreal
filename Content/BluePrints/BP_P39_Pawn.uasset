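; BP_P39_Pawn is a player-controlled aircraft pawn that constantly flies forward and steers by pitch and roll.
; Tick adds forward movement input along the actor's facing, then spins the Left and Right propellers through the shared RotatePropeller function.
; Pitch and Roll axis inputs apply clamped, delta-time-scaled local rotation using PlayerRotateSpeed.
; An older AddActorLocalOffset movement path using MoveSpeed is left disconnected.
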(event `self.ReceiveBeginPlay`)

(event `self.ReceiveTick`
  (params (DeltaSeconds :type "Float (single-precision)"))
  (`|ExecutionSequence`
    (:`then_0`
      (`self.AddMovementInput` (`self.GetActorForwardVector`)))
    (:`then_1`
      ;[1 1 1] 왼쪽 프로펠러 회전
      (`self.Rotate Propeller` (`self.Left`)))
    (:`then_2`
      ;[1 1 1] 오른쪽 프로펠러 회전
      (`self.Rotate Propeller` (`self.Right`)))))

(event `InputAxis|Pitch`
  (params (AxisValue :type "Float (single-precision)"))
  ;[1 1 1] Picth회전
  (`self.K2_AddActorLocalRotation` (`KismetMathLibrary.MakeRotator` 0.0 (* (`KismetMathLibrary.FClamp` AxisValue -1.0) (`GameplayStatics.GetWorldDeltaSeconds`) (`self.PlayerRotateSpeed`)))))

(event `InputAxis|Roll`
  (params (AxisValue :type "Float (single-precision)"))
  ;[1 1 1] Roll회전
  (`self.K2_AddActorLocalRotation` (`KismetMathLibrary.MakeRotator` (* (`KismetMathLibrary.FClamp` AxisValue -1.0) (`GameplayStatics.GetWorldDeltaSeconds`) (`self.PlayerRotateSpeed`)))))

(fn `Rotate Propeller`
  (params (Where :type "StaticMeshComponent Object Reference"))
  (`SceneComponent.K2_AddRelativeRotation` Where (`KismetMathLibrary.MakeRotator` (* (`GameplayStatics.GetWorldDeltaSeconds`) (`self.PropellerRotateSpeed`))) false false))

(fn `UserConstructionScript`)